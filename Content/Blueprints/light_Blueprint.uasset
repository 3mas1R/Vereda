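; An interactable light Blueprint that the player toggles with the E key while inside a trigger box.
; The box overlap enables and disables input and toggles a text render's visibility on entry and exit.
; Each press toggles the point light, and a FlipFlop alternates a timeline between play and reverse from end.
; The timeline update sets a static mesh's relative rotation to a fixed zero value.
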(event OnComponentBeginOverlap(Box)
  (params (OverlappedComponent :type Primitive%20Component%20Object%20Reference) (OtherActor :type Actor%20Object%20Reference) (OtherComp :type Primitive%20Component%20Object%20Reference) (OtherBodyIndex :type Integer) (bFromSweep :type Boolean) (SweepResult :type Hit%20Result%20Structure%20%28by%20ref%29))
  ;[1 1 1] disparador
  (Input|EnableInput (Game|GetPlayerController 0))
  (Rendering|ToggleVisibility (Variables|Default|GetTextRender) false))

(event OnComponentEndOverlap(Box)
  (params (OverlappedComponent :type Primitive%20Component%20Object%20Reference) (OtherActor :type Actor%20Object%20Reference) (OtherComp :type Primitive%20Component%20Object%20Reference) (OtherBodyIndex :type Integer))
  ;[1 1 1] disparador
  (Input|DisableInput (Game|GetPlayerController 0))
  (Rendering|ToggleVisibility (Variables|Default|GetTextRender) false))

(event EventBeginPlay)

(event Collision|EventActorBeginOverlap
  (params (OtherActor :type Actor%20Object%20Reference)))

(event EventTick
  (params (DeltaSeconds :type Float%20%28single-precision%29)))

(event Input|KeyboardEvents|E
  (params (Key :type Key%20Structure))
  ;[1 1 1] comando
  (:Pressed
    (Rendering|ToggleVisibility (Variables|Default|GetPointLight) false)
    (Utilities|FlowControl|FlipFlop
      (:A
        (Timeline|Línea%20de%20tiempo_0 Play
          (:Update
            (Transformation|SetRelativeRotation (Variables|Default|GetStaticMeshComponent03) "0, 0, 0" false false))))
      (:B
        (Timeline|Línea%20de%20tiempo_0 ReverseFromEnd)))))

(fn ConstructionScript)