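; BP_Puerta is a door that swings open and closed when triggered while something overlaps its collision box.
; Caja_Colision's begin and end overlap events set the CercaPuerta flag, with no check on which actor overlaps.
; The AbrirPuertaSeq event checks that flag, then a FlipFlop alternates between playing and reversing the AMT_Puerta timeline.
; The timeline's PuertaRotAmt track drives the yaw of the Puerta component's relative rotation.
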(event OnComponentBeginOverlap(Caja_Colision)
  (params (OverlappedComponent :type Primitive%20Component%20Object%20Reference) (OtherActor :type Actor%20Object%20Reference) (OtherComp :type Primitive%20Component%20Object%20Reference) (OtherBodyIndex :type Integer) (bFromSweep :type Boolean) (SweepResult :type Hit%20Result%20Structure%20%28by%20ref%29))
  ;[1 1 1] Detectar cuando se este cerca de la Puerta
  (Variables|Default|SetCerca_Puerta true))

(event OnComponentEndOverlap(Caja_Colision)
  (params (OverlappedComponent :type Primitive%20Component%20Object%20Reference) (OtherActor :type Actor%20Object%20Reference) (OtherComp :type Primitive%20Component%20Object%20Reference) (OtherBodyIndex :type Integer))
  ;[1 1 1] Detectar cuando se este cerca de la Puerta
  (Variables|Default|SetCerca_Puerta false))

(event Custom|AbrirPuertaSeq
  ;[1 1 1] Secuencia para Abrir Puerta
  (if (Variables|Default|GetCerca_Puerta)
    (Utilities|FlowControl|FlipFlop
      (:A
        (bind _puertarotamt (Timeline|AMT_Puerta Play)
          (:Update
            (Transformation|SetRelativeRotation (Variables|Default|GetPuerta) (Math|Rotator|MakeRotator 0.0 0.0 _puertarotamt) false false))))
      (:B
        (Timeline|AMT_Puerta Reverse)))))

(fn ConstructionScript)