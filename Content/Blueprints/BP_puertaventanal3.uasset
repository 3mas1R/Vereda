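; BP_puertaventanal3 is a sliding window door that the player operates with E while inside its overlap volume.
; Overlap enables player input, and E flip-flops the Desplazar_puerta timeline between play and reverse, sliding two meshes along relative X on separate tracks.
; Leaving disables input and, after a two-second delay, reverses the timeline from its end without checking door state or resetting the FlipFlop.
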(event OnComponentBeginOverlap(puertaventanal3)
  (params (OverlappedComponent :type Primitive%20Component%20Object%20Reference) (OtherActor :type Actor%20Object%20Reference) (OtherComp :type Primitive%20Component%20Object%20Reference) (OtherBodyIndex :type Integer) (bFromSweep :type Boolean) (SweepResult :type Hit%20Result%20Structure%20%28by%20ref%29))
  ;[1 1 1] Detectar cuando se este cerca de la Puerta
  (Input|EnableInput (Game|GetPlayerController 0)))

(event OnComponentEndOverlap(puertaventanal3)
  (params (OverlappedComponent :type Primitive%20Component%20Object%20Reference) (OtherActor :type Actor%20Object%20Reference) (OtherComp :type Primitive%20Component%20Object%20Reference) (OtherBodyIndex :type Integer))
  ;[1 1 1] Detectar cuando se este cerca de la Puerta
  (Input|DisableInput (Game|GetPlayerController 0))
  (Utilities|FlowControl|Delay 2.0)
  ;[1 1 1] Secuencia para Abrir Puerta
  (bind (_direction _newtrack_4 _newtrack_1) (Timeline|desplazar_puerta ReverseFromEnd)
    (:Update
      (Transformation|SetRelativeLocation (Variables|Default|GetStaticMeshComponent02) (Math|Vector|MakeVector (.x _newtrack_4) 0.0 0.0) false false)
      (Transformation|SetRelativeLocation (Variables|Default|GetStaticMeshComponent01) (Math|Vector|MakeVector (.x _newtrack_1) 0.0 0.0) false false))))

(event EventBeginPlay)

(event Collision|EventActorBeginOverlap
  (params (OtherActor :type Actor%20Object%20Reference)))

(event EventTick
  (params (DeltaSeconds :type Float%20%28single-precision%29)))

(event Input|KeyboardEvents|E
  (params (Key :type Key%20Structure))
  ;[1 1 1] Secuencia para Abrir Puerta
  (:Pressed
    (Utilities|FlowControl|FlipFlop
      (:A
        (bind (_direction _newtrack_4 _newtrack_1) (Timeline|desplazar_puerta Play)
          (:Update
            (Transformation|SetRelativeLocation (Variables|Default|GetStaticMeshComponent02) (Math|Vector|MakeVector (.x _newtrack_4) 0.0 0.0) false false)
            (Transformation|SetRelativeLocation (Variables|Default|GetStaticMeshComponent01) (Math|Vector|MakeVector (.x _newtrack_1) 0.0 0.0) false false))))
      (:B
        (Timeline|desplazar_puerta Reverse)))))

(fn ConstructionScript)