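; Interactive water faucet actor that the player turns on and off with the E key.
; Entering the Box trigger enables input for player 0, and leaving disables it without stopping the water.
; E activates or deactivates the Water1 particle component, which gets the P_Water template at BeginPlay and starts off.
; GrifoAbierto works as a "next press opens" flag, set true on every overlap begin regardless of water state.
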(event OnComponentBeginOverlap(Box)
  (params (OverlappedComponent :type Primitive%20Component%20Object%20Reference) (OtherActor :type Actor%20Object%20Reference) (OtherComp :type Primitive%20Component%20Object%20Reference) (OtherBodyIndex :type Integer) (bFromSweep :type Boolean) (SweepResult :type Hit%20Result%20Structure%20%28by%20ref%29))
  (Input|EnableInput (Game|GetPlayerController 0))
  (Variables|Default|Setgrifo_abierto true))

(event OnComponentEndOverlap(Box)
  (params (OverlappedComponent :type Primitive%20Component%20Object%20Reference) (OtherActor :type Actor%20Object%20Reference) (OtherComp :type Primitive%20Component%20Object%20Reference) (OtherBodyIndex :type Integer))
  (Input|DisableInput (Game|GetPlayerController 0))
  (Variables|Default|Setgrifo_abierto false))

(event EventBeginPlay
  (bind _water1 (Variables|Default|GetWater1))
  (Effects|Components|ParticleSystem|SetTemplate _water1 "/Game/Particles/P_Water.P_Water")
  (Components|Activation|Deactivate _water1))

(event Input|KeyboardEvents|E
  (params (Key :type Key%20Structure))
  (bind _water1 (Variables|Default|GetWater1))
  (:Pressed
    (if (Variables|Default|Getgrifo_abierto)
      (Components|Activation|Activate _water1 false)
      (Variables|Default|Setgrifo_abierto false)
      (else
        (Components|Activation|Deactivate _water1)
        (Variables|Default|Setgrifo_abierto true)))))

(fn ConstructionScript)