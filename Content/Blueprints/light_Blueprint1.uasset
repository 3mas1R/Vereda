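; Light switch actor that the player toggles with E while standing inside its Box trigger.
; Overlapping the Box enables input from the first player controller, and leaving it disables input.
; A FlipFlop alternates the PointLight intensity between on and off.
; It also plays or reverses a timeline that drives the roll of StaticMeshComponent03, animating it with the toggle.
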(event OnComponentBeginOverlap(Box)
  (params (OverlappedComponent :type Primitive%20Component%20Object%20Reference) (OtherActor :type Actor%20Object%20Reference) (OtherComp :type Primitive%20Component%20Object%20Reference) (OtherBodyIndex :type Integer) (bFromSweep :type Boolean) (SweepResult :type Hit%20Result%20Structure%20%28by%20ref%29))
  ;[1 1 1] disparador
  (Input|EnableInput (Game|GetPlayerController 0)))

(event OnComponentEndOverlap(Box)
  (params (OverlappedComponent :type Primitive%20Component%20Object%20Reference) (OtherActor :type Actor%20Object%20Reference) (OtherComp :type Primitive%20Component%20Object%20Reference) (OtherBodyIndex :type Integer))
  ;[1 1 1] disparador
  (Input|DisableInput (Game|GetPlayerController 0)))

(event EventBeginPlay)

(event Collision|EventActorBeginOverlap
  (params (OtherActor :type Actor%20Object%20Reference)))

(event EventTick
  (params (DeltaSeconds :type Float%20%28single-precision%29)))

(event Input|KeyboardEvents|E
  (params (Key :type Key%20Structure))
  (bind _pointlight (Variables|Default|GetPointLight))
  ;[1 1 1] comando
  (:Pressed
    (Utilities|FlowControl|FlipFlop
      (:A
        (Rendering|Components|Light|SetIntensity _pointlight 5e+03)
        (bind _newtrack_4 (Timeline|Línea%20de%20tiempo_0 Play)
          (:Update
            (Transformation|SetRelativeRotation (Variables|Default|GetStaticMeshComponent03) (Math|Rotator|MakeRotator _newtrack_4 0.0 0.0) false false))))
      (:B
        (Rendering|Components|Light|SetIntensity _pointlight 0.0)
        (Timeline|Línea%20de%20tiempo_0 Reverse)))))

(fn ConstructionScript)